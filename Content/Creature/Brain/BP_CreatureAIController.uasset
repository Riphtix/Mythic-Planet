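; AI controller for BP_CreaturePawn that walks the creature toward target locations the pawn reports.
; On possess it binds to the pawn's target-location update, storing each new location and calling DecideToMove.
; DecideToMove passes a coin flip to start the move and set a looping, random-interval timer on itself; a failed flip leaves movement and timer untouched.
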(event `self.ReceivePossess`
  (params (PossessedPawn :type "Pawn Object Reference"))
  (bind _asbp_creature_pawn (cast `/Game/Creature/Blueprints/BP_CreaturePawn` PossessedPawn))
  (add `/Game/Creature/Blueprints/BP_CreaturePawn.OnTargetLocationUpdated` _asbp_creature_pawn (delegate `Event Begin Walk Movement`)))

(event `Event Begin Walk Movement`
  (params (NewTargetLocation :type "Vector Structure"))
  (set `self.Target Location` NewTargetLocation)
  (`self.DecideToMove`))

(fn `DecideToMove`
  (if (> (`KismetMathLibrary.RandomFloatInRange` 0.0 1.0) 0.5)
    (`self.MoveToTargetLocation`)
    (`KismetSystemLibrary.K2_SetTimer` null "DecideToMove" (`KismetMathLibrary.RandomFloatInRange` 5.0 15.0) true)))

(fn `MoveToTargetLocation`
  (`self.MoveToLocation` (`self.Target Location`) -1.0 true true false true null))

(fn `UserConstructionScript`)