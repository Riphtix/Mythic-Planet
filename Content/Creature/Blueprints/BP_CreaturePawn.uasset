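; Creature pawn that randomizes a genetics struct at BeginPlay and derives speed and favored movement mode from it.
; Normalized walk/fly/swim weights blend MaxSpeed and set the default mode.
; A self-rescheduling timer re-picks the mode from biome weights, water state and a ground trace, with occasional random choice, then schedules a random navigable target broadcast through OnTargetLocationUpdated.
; ExecuteMovement is an empty switch, and debug drawing shows traces and targets.
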(event `self.ReceiveBeginPlay`
  (`self.InitializeGenes`)
  (`self.ApplyGenetics`)
  (`self.DecideMovementMode`)
  (`self.RunAIDebugFunctions`))

(event `self.ReceiveTick`
  (params (DeltaSeconds :type "Float (single-precision)")))

(fn `ApplyGenetics`
  (bind (_walkingspeed _runningspeed _flyingspeed _swimmingspeed _oxygensourcetype _temperaturefavor _humidityfavor _hypothermiatemperature _hyperthermiatemperature _extrathermalsurvivalduration _bloodtemperature _foodpreference _preferredmovementbiome) (break `/Game/Creature/Genes/G_EnvirionmentalAttributes` (`.EnvironmentalAttributes_6_566039D844D90EDACBC513BFFD8608E4` (break `/Game/Creature/Genes/G_Genetics` (`self.Genetics`)))))
  (`self.NormalizePreferredBiome`)
  (`self.DetermineMovementType`)
  ; Apply Movement
  (set `FloatingPawnMovement.MaxSpeed` (+ (* _walkingspeed (.x _preferredmovementbiome)) (* _flyingspeed (.y _preferredmovementbiome)) (* _swimmingspeed (.z _preferredmovementbiome))) (`self.MovementComponent`)))

(fn `CheckIsGrounded`
  (locals (ZOffset :type "Float (double-precision)" :default 15.0) (EndPoint :type "Float (double-precision)"))
  (bind _returnvalue_location (`KismetMathLibrary.BreakTransform` (`self.GetTransform`)))
  (bind _output_get (set `local.EndPoint` (- (.z _returnvalue_location) (`local.ZOffset`))))
  (bind (_outhit _returnvalue) (`KismetSystemLibrary.LineTraceSingle` :`Start` _returnvalue_location :`End` (`KismetMathLibrary.MakeVector` (.x _returnvalue_location) (.y _returnvalue_location) _output_get) :`TraceChannel` "TraceTypeQuery1" :`DrawDebugType` "ForDuration" :`TraceColor` (struct :`R` 0.188703 :`G` 1.0 :`B` 0.788491 :`A` 1.0)))
  (set `self.IsGrounded` _returnvalue))

(fn `DecideMovementMode`
  (locals (ValidMovementModes :type "Array of /Game/Creature/Genes/E_MovementMode Enum") (MovementTypeDecisionTimer :type "Float (double-precision)") (`Start Movement Timer` :type "Float (double-precision)"))
  (bind _validmovementmodes (`local.ValidMovementModes`))
  (bind _isgrounded (`self.IsGrounded`))
  (bind (_walkingspeed _runningspeed _flyingspeed _swimmingspeed _oxygensourcetype _temperaturefavor _humidityfavor _hypothermiatemperature _hyperthermiatemperature _extrathermalsurvivalduration _bloodtemperature _foodpreference _preferredmovementbiome _movementstylefavor) (break `/Game/Creature/Genes/G_EnvirionmentalAttributes` (`.EnvironmentalAttributes_6_566039D844D90EDACBC513BFFD8608E4` (break `/Game/Creature/Genes/G_Genetics` (`self.Genetics`)))))
  (bind _returnvalue (>= (.y _preferredmovementbiome) 0.5))
  (bind _returnvalue_2 (and (>= (.z _preferredmovementbiome) 0.2) (`self.IsInWater`)))
  (`self.NormalizePreferredBiome`)
  (`self.CheckIsGrounded` :!label _label)
  ; Valid Movement Modes
  (if _returnvalue_2
    (`KismetArrayLibrary.Array_AddUnique` _validmovementmodes "NewEnumerator2")
    (elif _returnvalue
      (`KismetArrayLibrary.Array_AddUnique` _validmovementmodes "NewEnumerator1")
      (elif _isgrounded
        (`KismetArrayLibrary.Array_AddUnique` _validmovementmodes "NewEnumerator0")
        (else
          (`KismetArrayLibrary.Array_RemoveItem` _validmovementmodes "NewEnumerator0")))))
  (if (< (`KismetMathLibrary.RandomFloatInRange` 0.0 1.0) 0.2)
    (set `self.CurrentMovementMode` (`KismetArrayLibrary.Array_Random` _validmovementmodes))
    (elif _returnvalue_2
      (set `self.CurrentMovementMode` "NewEnumerator2")
      (elif _returnvalue
        (set `self.CurrentMovementMode` "NewEnumerator1")
        (elif _isgrounded
          (set `self.CurrentMovementMode` _movementstylefavor)
          (else
            (goto _label))))))
  (bind _output_get (set `local.MovementTypeDecisionTimer` (`KismetMathLibrary.RandomFloatInRange` 1.0 5.0)))
  (`KismetSystemLibrary.K2_SetTimer` null "DecideMovementMode" _output_get)
  (bind _output_get_2 (set `local.Start Movement Timer` (`KismetMathLibrary.RandomFloatInRange` 0.0 0.5)))
  (`KismetSystemLibrary.K2_SetTimer` null "SelectNewTarget" _output_get_2))

(fn `DetermineMovementType`
  (locals (FinalMax :type "Float (double-precision)") (MovementIndex :type Integer))
  (bind _finalmax (`local.FinalMax`))
  (bind (_coreattributes _environmentalattributes _physicalattributes _socialattributes _perceptionattributes) (break `/Game/Creature/Genes/G_Genetics` (`self.Genetics`)))
  (bind (_walkingspeed _runningspeed _flyingspeed _swimmingspeed _oxygensourcetype _temperaturefavor _humidityfavor _hypothermiatemperature _hyperthermiatemperature _extrathermalsurvivalduration _bloodtemperature _foodpreference _preferredmovementbiome) (break `/Game/Creature/Genes/G_EnvirionmentalAttributes` _environmentalattributes))
  (bind _x (.x _preferredmovementbiome))
  (bind _y (.y _preferredmovementbiome))
  ; Find Main Preference
  (set `local.FinalMax` (`KismetMathLibrary.FMax` (`KismetMathLibrary.FMax` _x _y) (.z _preferredmovementbiome)))
  ; Use main preference to determine the genetic default movement choice
  (if (== _x _finalmax)
    (set `local.MovementIndex` 0)
    (elif (== _y _finalmax)
      (set `local.MovementIndex` 1)
      (else
        (set `local.MovementIndex` 2))))
  ; Set the genetic default movement choice
  (bind _output_get (set `self.CurrentMovementMode` (select `int` (`local.MovementIndex`) :`0` "NewEnumerator0" :`1` "NewEnumerator1" :`2` "NewEnumerator2" :!type "/Game/Creature/Genes/E_MovementMode Enum")))
  (`KismetSystemLibrary.PrintString` (`KismetStringLibrary.Concat_StrStr` "Initial Movement Mode: " (`|GetEnumeratorNameAsString` _output_get)))
  (set `self.Genetics` (make `/Game/Creature/Genes/G_Genetics` _coreattributes (make `/Game/Creature/Genes/G_EnvirionmentalAttributes` _walkingspeed _runningspeed _flyingspeed _swimmingspeed _oxygensourcetype _temperaturefavor _humidityfavor _hypothermiatemperature _hyperthermiatemperature _extrathermalsurvivalduration _bloodtemperature _foodpreference _preferredmovementbiome _output_get) _physicalattributes _socialattributes _perceptionattributes)))

(fn `ExecuteMovement`
  (params (`Target Location` :type "Vector Structure"))
  (switch `/Game/Creature/Genes/E_MovementMode` (`self.CurrentMovementMode`)))

(fn `InitializeGenes`
  (bind _returnvalue (`KismetMathLibrary.RandomFloatInRange` 1.0 5.0))
  (bind _returnvalue_2 (`KismetMathLibrary.RandomFloatInRange` -100.0 100.0))
  (set `self.Genetics` (make `/Game/Creature/Genes/G_Genetics` (make `/Game/Creature/Genes/G_CoreAttributes` (`KismetMathLibrary.RandomFloatInRange` 5.0 100.0) (`KismetMathLibrary.RandomIntegerInRange` 0 1) (`KismetMathLibrary.RandomIntegerInRange` 0 11) 0 (`KismetMathLibrary.RandomFloatInRange` 0.0 1.0) (`KismetMathLibrary.RandomFloatInRange` 0.0 1.0) (`KismetMathLibrary.RandomFloatInRange` 50.0 150.0) (`KismetMathLibrary.RandomFloatInRange` 20.0 100.0) (`KismetMathLibrary.RandomFloatInRange` 20.0 100.0) (`KismetMathLibrary.RandomFloatInRange` 20.0 100.0) (`KismetMathLibrary.RandomFloatInRange` 20.0 100.0)) (make `/Game/Creature/Genes/G_EnvirionmentalAttributes` _returnvalue (`KismetMathLibrary.RandomFloatInRange` (+ _returnvalue 2.0) (+ _returnvalue 5.0)) (`KismetMathLibrary.RandomFloatInRange` 5.0 15.0) (`KismetMathLibrary.RandomFloatInRange` 2.0 15.0) (`KismetMathLibrary.RandomIntegerInRange` 0 3) _returnvalue_2 (`KismetMathLibrary.RandomFloatInRange` 0.0 1.0) (- _returnvalue_2 (`KismetMathLibrary.RandomFloatInRange` 30.0 50.0)) (+ _returnvalue_2 (`KismetMathLibrary.RandomFloatInRange` 30.0 50.0)) (`KismetMathLibrary.RandomFloatInRange` 10.0 100.0) (`KismetMathLibrary.RandomFloatInRange` 0.0 1.0) (`KismetMathLibrary.RandomIntegerInRange` 0 3) (`KismetMathLibrary.MakeVector` (`KismetMathLibrary.RandomFloatInRange` 0.0 1.0) (`KismetMathLibrary.RandomFloatInRange` 0.0 1.0) (`KismetMathLibrary.RandomFloatInRange` 0.0 1.0))) (make `/Game/Creature/Genes/G_PhysicalAttributes` (`KismetMathLibrary.MakeVector` (`KismetMathLibrary.RandomFloatInRange` 0.0 1.0) (`KismetMathLibrary.RandomFloatInRange` 0.0 1.0) (`KismetMathLibrary.RandomFloatInRange` 0.0 1.0)) (`KismetMathLibrary.RandomIntegerInRange` 0 10) (`KismetMathLibrary.RandomIntegerInRange` 0 1) (`KismetMathLibrary.RandomFloatInRange` 0.0 1.0) (`KismetMathLibrary.RandomFloatInRange` 0.5 5.0) (`KismetMathLibrary.RandomFloatInRange` 0.01 0.1)) (make `/Game/Creature/Genes/G_SocialAttributes` (`KismetMathLibrary.RandomIntegerInRange` 0 1) (`KismetMathLibrary.RandomIntegerInRange` 0 1) (`KismetMathLibrary.RandomFloatInRange` 0.0 1.0) (`KismetMathLibrary.RandomFloatInRange` 0.0 1.0) (`KismetMathLibrary.RandomFloatInRange` 0.0 1.0) (`KismetMathLibrary.RandomFloatInRange` 0.1 1.0)) (make `/Game/Creature/Genes/G_PerceptionAttributes` (`KismetMathLibrary.RandomFloatInRange` 0.0 1.0) (`KismetMathLibrary.RandomFloatInRange` 0.0 1.0) (`KismetMathLibrary.RandomFloatInRange` 0.0 1.0) (`KismetMathLibrary.RandomIntegerInRange` 0 1) (`KismetMathLibrary.RandomFloatInRange` 0.0 1.0)))))

(fn `NormalizePreferredBiome`
  (locals (Total :type "Float (double-precision)") (SafeTotal :type "Float (double-precision)"))
  (bind (_coreattributes _environmentalattributes _physicalattributes _socialattributes _perceptionattributes) (break `/Game/Creature/Genes/G_Genetics` (`self.Genetics`)))
  (bind (_walkingspeed _runningspeed _flyingspeed _swimmingspeed _oxygensourcetype _temperaturefavor _humidityfavor _hypothermiatemperature _hyperthermiatemperature _extrathermalsurvivalduration _bloodtemperature _foodpreference _preferredmovementbiome _movementstylefavor) (break `/Game/Creature/Genes/G_EnvirionmentalAttributes` _environmentalattributes))
  (bind _x (.x _preferredmovementbiome))
  (bind _y (.y _preferredmovementbiome))
  (bind _z (.z _preferredmovementbiome))
  ; Normalize the preferred movement values
  (bind _output_get (set `local.Total` (+ _x _y _z)))
  (if (== _output_get 0.0)
    (set `local.SafeTotal` 1.0)
    (else
      (bind _output_get_2 (set `local.SafeTotal` _output_get))))
  (set `self.Genetics` (make `/Game/Creature/Genes/G_Genetics` _coreattributes (make `/Game/Creature/Genes/G_EnvirionmentalAttributes` _walkingspeed _runningspeed _flyingspeed _swimmingspeed _oxygensourcetype _temperaturefavor _humidityfavor _hypothermiatemperature _hyperthermiatemperature _extrathermalsurvivalduration _bloodtemperature _foodpreference (`KismetMathLibrary.MakeVector` (/ _x _output_get_2) (/ _y _output_get_2) (/ _z _output_get_2)) _movementstylefavor) _physicalattributes _socialattributes _perceptionattributes)))

(fn `RunAIDebugFunctions`
  (`KismetSystemLibrary.DrawDebugLine` (`SceneComponent.K2_GetComponentLocation` (`self.DefaultSceneRoot`)) (`self.Target Location`) (struct :`G` 0.598958 :`B` 0.12096 :`A` 1.0) 1.0 1.0)
  (`KismetSystemLibrary.K2_SetTimer` null "RunAIDebugFunctions" 1.0))

(fn `SelectNewTarget`
  (bind _returnvalue_location (`KismetMathLibrary.BreakTransform` (`self.GetTransform`)))
  (bind _randomlocation (`NavigationSystemV1.K2_GetRandomLocationInNavigableRadius` _returnvalue_location (`self.SearchRadius`) null null))
  (bind _output_get (set `self.Target Location` _randomlocation))
  (`self.OnTargetLocationUpdated` _output_get))

(fn `UserConstructionScript`)