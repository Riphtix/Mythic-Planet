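; BP_Creature is a creature that randomizes its full genetics on BeginPlay and derives movement from them.
; ApplyGenetics normalizes walk/fly/swim biome preferences, stores the strongest as default style, and sets MaxSpeed from their weighted speeds.
; DecideMovementMode reschedules itself on a random timer, choosing randomly or by water state and preference, without updating speed.
; MoveCreature, SenseEnvironment, EatFood and Reproduce are empty stubs.
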(event `self.ReceiveBeginPlay`
  (`self.InitializeGenes`)
  (`self.ApplyGenetics`)
  (`self.DecideMovementMode`))

(event `self.ReceiveTick`
  (params (DeltaSeconds :type "Float (single-precision)")))

(fn `ApplyGenetics`
  (bind (_walkingspeed _runningspeed _flyingspeed _swimmingspeed _oxygensourcetype _temperaturefavor _humidityfavor _hypothermiatemperature _hyperthermiatemperature _extrathermalsurvivalduration _bloodtemperature _foodpreference _preferredmovementbiome) (break `/Game/Creature/Genes/G_EnvirionmentalAttributes` (`.EnvironmentalAttributes_6_566039D844D90EDACBC513BFFD8608E4` (break `/Game/Creature/Genes/G_Genetics` (`self.Genetics`)))))
  (`self.NormalizePreferredBiome`)
  (`self.DetermineMovementType`)
  ; Apply Movement
  (set `FloatingPawnMovement.MaxSpeed` (+ (* _walkingspeed (.x _preferredmovementbiome)) (* _flyingspeed (.y _preferredmovementbiome)) (* _swimmingspeed (.z _preferredmovementbiome))) (`self.MovementComponent`)))

(fn `DecideMovementMode`
  (bind (_walkingspeed _runningspeed _flyingspeed _swimmingspeed _oxygensourcetype _temperaturefavor _humidityfavor _hypothermiatemperature _hyperthermiatemperature _extrathermalsurvivalduration _bloodtemperature _foodpreference _preferredmovementbiome _movementstylefavor) (break `/Game/Creature/Genes/G_EnvirionmentalAttributes` (`.EnvironmentalAttributes_6_566039D844D90EDACBC513BFFD8608E4` (break `/Game/Creature/Genes/G_Genetics` (`self.Genetics`)))))
  (if (< (`KismetMathLibrary.RandomFloatInRange` 0.0 1.0) 0.2)
    (bind _output_get (set `self.CurrentMovementMode` (select `int` (`KismetMathLibrary.RandomIntegerInRange` 0 2) :`0` "NewEnumerator0" :`1` "NewEnumerator1" :`2` "NewEnumerator2" :!type "/Game/Creature/Genes/E_MovementMode Enum")))
    (`KismetSystemLibrary.PrintString` (`KismetStringLibrary.Concat_StrStr` "Switched to " (`|GetEnumeratorNameAsString` _output_get)))
    (elif (and (>= (.z _preferredmovementbiome) 0.2) (`self.IsInWater`))
      (bind _output_get_2 (set `self.CurrentMovementMode` "NewEnumerator2"))
      (`KismetSystemLibrary.PrintString` (`KismetStringLibrary.Concat_StrStr` "Switched to " (`|GetEnumeratorNameAsString` _output_get_2)))
      (elif (>= (.y _preferredmovementbiome) 0.2)
        (bind _output_get_3 (set `self.CurrentMovementMode` "NewEnumerator1"))
        (`KismetSystemLibrary.PrintString` (`KismetStringLibrary.Concat_StrStr` "Switched to " (`|GetEnumeratorNameAsString` _output_get_3)))
        (else
          (bind _output_get_4 (set `self.CurrentMovementMode` _movementstylefavor))
          (`KismetSystemLibrary.PrintString` (`KismetStringLibrary.Concat_StrStr` "Switched to " (`|GetEnumeratorNameAsString` _output_get_4)))))))
  (bind _output_get_5 (set `self.Movement Type Decision Timer` (`KismetMathLibrary.RandomFloatInRange` 1.0 5.0)))
  (`KismetSystemLibrary.K2_SetTimer` null "DecideMovementMode" _output_get_5))

(fn `DetermineMovementType`
  (locals (FinalMax :type "Float (double-precision)" :default 0.0) (MovementIndex :type Integer))
  (bind _finalmax (`local.FinalMax`))
  (bind (_coreattributes _environmentalattributes _physicalattributes _socialattributes _perceptionattributes) (break `/Game/Creature/Genes/G_Genetics` (`self.Genetics`)))
  (bind (_walkingspeed _runningspeed _flyingspeed _swimmingspeed _oxygensourcetype _temperaturefavor _humidityfavor _hypothermiatemperature _hyperthermiatemperature _extrathermalsurvivalduration _bloodtemperature _foodpreference _preferredmovementbiome) (break `/Game/Creature/Genes/G_EnvirionmentalAttributes` _environmentalattributes))
  (bind _x (.x _preferredmovementbiome))
  (bind _y (.y _preferredmovementbiome))
  ; Find Main Preference
  (set `local.FinalMax` (`KismetMathLibrary.FMax` (`KismetMathLibrary.FMax` _x _y) (.z _preferredmovementbiome)))
  ; Use main preference to determine the genetic default movement choice
  (if (== _x _finalmax)
    (set `local.MovementIndex` 0)
    (elif (== _y _finalmax)
      (set `local.MovementIndex` 1)
      (else
        (set `local.MovementIndex` 2))))
  ; Set the genetic default movement choice
  (bind _output_get (set `self.CurrentMovementMode` (select `int` (`local.MovementIndex`) :`0` "NewEnumerator0" :`1` "NewEnumerator1" :`2` "NewEnumerator2" :!type "/Game/Creature/Genes/E_MovementMode Enum")))
  (`KismetSystemLibrary.PrintString` (`KismetStringLibrary.Concat_StrStr` "Initial Movement Mode: " (`|GetEnumeratorNameAsString` _output_get)))
  (set `self.Genetics` (make `/Game/Creature/Genes/G_Genetics` _coreattributes (make `/Game/Creature/Genes/G_EnvirionmentalAttributes` _walkingspeed _runningspeed _flyingspeed _swimmingspeed _oxygensourcetype _temperaturefavor _humidityfavor _hypothermiatemperature _hyperthermiatemperature _extrathermalsurvivalduration _bloodtemperature _foodpreference _preferredmovementbiome _output_get) _physicalattributes _socialattributes _perceptionattributes)))

(fn `EatFood`)

(fn `InitializeGenes`
  (bind _returnvalue (`KismetMathLibrary.RandomFloatInRange` 1.0 5.0))
  (bind _returnvalue_2 (`KismetMathLibrary.RandomFloatInRange` -100.0 100.0))
  (set `self.Genetics` (make `/Game/Creature/Genes/G_Genetics` (make `/Game/Creature/Genes/G_CoreAttributes` (`KismetMathLibrary.RandomFloatInRange` 5.0 100.0) (`KismetMathLibrary.RandomIntegerInRange` 0 1) (`KismetMathLibrary.RandomIntegerInRange` 0 11) 0 (`KismetMathLibrary.RandomFloatInRange` 0.0 1.0) (`KismetMathLibrary.RandomFloatInRange` 0.0 1.0) (`KismetMathLibrary.RandomFloatInRange` 50.0 150.0) (`KismetMathLibrary.RandomFloatInRange` 20.0 100.0) (`KismetMathLibrary.RandomFloatInRange` 20.0 100.0) (`KismetMathLibrary.RandomFloatInRange` 20.0 100.0) (`KismetMathLibrary.RandomFloatInRange` 20.0 100.0)) (make `/Game/Creature/Genes/G_EnvirionmentalAttributes` _returnvalue (`KismetMathLibrary.RandomFloatInRange` (+ _returnvalue 2.0) (+ _returnvalue 5.0)) (`KismetMathLibrary.RandomFloatInRange` 5.0 15.0) (`KismetMathLibrary.RandomFloatInRange` 2.0 15.0) (`KismetMathLibrary.RandomIntegerInRange` 0 3) _returnvalue_2 (`KismetMathLibrary.RandomFloatInRange` 0.0 1.0) (- _returnvalue_2 (`KismetMathLibrary.RandomFloatInRange` 30.0 50.0)) (+ _returnvalue_2 (`KismetMathLibrary.RandomFloatInRange` 30.0 50.0)) (`KismetMathLibrary.RandomFloatInRange` 10.0 100.0) (`KismetMathLibrary.RandomFloatInRange` 0.0 1.0) (`KismetMathLibrary.RandomIntegerInRange` 0 3) (`KismetMathLibrary.MakeVector` (`KismetMathLibrary.RandomFloatInRange` 0.0 1.0) (`KismetMathLibrary.RandomFloatInRange` 0.0 1.0) (`KismetMathLibrary.RandomFloatInRange` 0.0 1.0))) (make `/Game/Creature/Genes/G_PhysicalAttributes` (`KismetMathLibrary.MakeVector` (`KismetMathLibrary.RandomFloatInRange` 0.0 1.0) (`KismetMathLibrary.RandomFloatInRange` 0.0 1.0) (`KismetMathLibrary.RandomFloatInRange` 0.0 1.0)) (`KismetMathLibrary.RandomIntegerInRange` 0 10) (`KismetMathLibrary.RandomIntegerInRange` 0 1) (`KismetMathLibrary.RandomFloatInRange` 0.0 1.0) (`KismetMathLibrary.RandomFloatInRange` 0.5 5.0) (`KismetMathLibrary.RandomFloatInRange` 0.01 0.1)) (make `/Game/Creature/Genes/G_SocialAttributes` (`KismetMathLibrary.RandomIntegerInRange` 0 1) (`KismetMathLibrary.RandomIntegerInRange` 0 1) (`KismetMathLibrary.RandomFloatInRange` 0.0 1.0) (`KismetMathLibrary.RandomFloatInRange` 0.0 1.0) (`KismetMathLibrary.RandomFloatInRange` 0.0 1.0) (`KismetMathLibrary.RandomFloatInRange` 0.1 1.0)) (make `/Game/Creature/Genes/G_PerceptionAttributes` (`KismetMathLibrary.RandomFloatInRange` 0.0 1.0) (`KismetMathLibrary.RandomFloatInRange` 0.0 1.0) (`KismetMathLibrary.RandomFloatInRange` 0.0 1.0) (`KismetMathLibrary.RandomIntegerInRange` 0 1) (`KismetMathLibrary.RandomFloatInRange` 0.0 1.0)))))

(fn `MoveCreature`)

(fn `NormalizePreferredBiome`
  (bind (_coreattributes _environmentalattributes _physicalattributes _socialattributes _perceptionattributes) (break `/Game/Creature/Genes/G_Genetics` (`self.Genetics`)))
  (bind (_walkingspeed _runningspeed _flyingspeed _swimmingspeed _oxygensourcetype _temperaturefavor _humidityfavor _hypothermiatemperature _hyperthermiatemperature _extrathermalsurvivalduration _bloodtemperature _foodpreference _preferredmovementbiome _movementstylefavor) (break `/Game/Creature/Genes/G_EnvirionmentalAttributes` _environmentalattributes))
  (bind _x (.x _preferredmovementbiome))
  (bind _y (.y _preferredmovementbiome))
  (bind _z (.z _preferredmovementbiome))
  ; Normalize the preferred movement values
  (bind _output_get (set `self.Total` (+ _x _y _z)))
  (if (== _output_get 0.0)
    (set `self.SafeTotal` 1.0)
    (else
      (bind _output_get_2 (set `self.SafeTotal` _output_get))))
  (set `self.Genetics` (make `/Game/Creature/Genes/G_Genetics` _coreattributes (make `/Game/Creature/Genes/G_EnvirionmentalAttributes` _walkingspeed _runningspeed _flyingspeed _swimmingspeed _oxygensourcetype _temperaturefavor _humidityfavor _hypothermiatemperature _hyperthermiatemperature _extrathermalsurvivalduration _bloodtemperature _foodpreference (`KismetMathLibrary.MakeVector` (/ _x _output_get_2) (/ _y _output_get_2) (/ _z _output_get_2)) _movementstylefavor) _physicalattributes _socialattributes _perceptionattributes)))

(fn `Reproduce`)

(fn `SenseEnvironment`)

(fn `UserConstructionScript`)